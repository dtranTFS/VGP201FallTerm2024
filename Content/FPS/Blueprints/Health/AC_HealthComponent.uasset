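; Reusable health component for FPS actors that tracks current health between configurable minimum and maximum bounds.
; On BeginPlay, Init applies the bounds and fills health to maximum.
; Damage, Heal and HealFull route through SetHealth, which clamps every write to those bounds.
; Query functions expose current health, a 0–1 normalized value and a death check at zero or below, with no events broadcast on change.
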(event EventBeginPlay
  (CallFunction|Init (Variables|Setup|GetMinHealth) (Variables|Setup|GetMaxHealth)))

(fn Heal
  (params (Heal%20Amt :type Float%20%28double-precision%29))
  (CallFunction|SetHealth (CallFunction|ClampHealth (+ (CallFunction|GetHealth) Heal%20Amt))))

(fn Damage
  (params (Damage%20Amt :type Float%20%28double-precision%29))
  (CallFunction|SetHealth (CallFunction|ClampHealth (- (CallFunction|GetHealth) Damage%20Amt))))

(fn GetHealth
  (return (Variables|Setup|GetHealth)))

(fn SetHealth
  (params (New%20Health :type Float%20%28double-precision%29))
  (Variables|Setup|SetHealth (CallFunction|ClampHealth New%20Health)))

(fn HealFull
  (CallFunction|Heal (Variables|Setup|GetMaxHealth)))

(fn IsDead
  (return (<= (CallFunction|GetHealth) 0.0)))

(fn GetNormalizedHealth
  (return (Math|Float|Clamp(Float) (/ (Variables|Setup|GetHealth) (Variables|Setup|GetMaxHealth)))))

(fn Init
  (params (Min%20Health :type Float%20%28double-precision%29) (Max%20Health :type Float%20%28double-precision%29))
  (Variables|Setup|SetMinHealth Min%20Health)
  (bind _output_get (Variables|Setup|SetMaxHealth Max%20Health))
  (CallFunction|SetHealth _output_get))

(fn ClampHealth
  (params (Value :type Float%20%28double-precision%29))
  (return (Math|Float|Clamp(Float) Value (Variables|Setup|GetMinHealth) (Variables|Setup|GetMaxHealth))))